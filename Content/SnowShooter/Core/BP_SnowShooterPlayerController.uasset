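; Player controller for SnowShooter that opens team selection and passes the player's team to the controlled character.
; On BeginPlay, if it is player controller 0, it shows the WBP_PickTeam widget with UI-only input and a visible cursor.
; A custom event reads TeamIndex from SnowShooterPlayerState and forwards it to a custom event on the possessed FirstPersonCharacter.
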(event Custom|CustomEvent_0
  (bind _asfirst_person_character (Utilities|Casting|CastToFirstPersonCharacter (Pawn|GetControlledPawn)))
  (Default|CustomEvent0 _asfirst_person_character (Variables|/Script/SnowShooter.SnowShooterPlayerState|GetTeamIndex (.AsSnow%20Shooter%20Player%20State (Utilities|Casting|CastToSnowShooterPlayerState (Variables|Default|GetPlayerState))))))

(event EventBeginPlay
  (bind _self self)
  (if (== (Game|GetPlayerController 0) _self)
    (bind _returnvalue (UserInterface|CreateWidget "/Game/SnowShooter/UI/WBP_PickTeam.WBP_PickTeam_C" _self))
    (UserInterface|Viewport|AddtoViewport _returnvalue 0)
    (Input|SetInputModeUIOnly _self 0 "DoNotLock")
    (Variables|Default|SetbShowMouseCursor true)))

(fn ConstructionScript)