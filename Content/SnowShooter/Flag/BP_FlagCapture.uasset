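; BP_FlagCapture is a capture-point flag in SnowShooter that assigns itself to the team with more unfrozen players inside its sphere.
; Each server tick tallies overlapping characters by player-state team and switches ownership immediately on a majority, leaving it unchanged on a tie.
; It writes the owner into the game state's FlagOccupiers array at FlagIndex and recolors the cube, with the material change running only on authority.
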(event EventBeginPlay)

(event Collision|EventActorBeginOverlap
  (params (OtherActor :type Actor%20Object%20Reference)))

(event EventTick
  (params (DeltaSeconds :type Float%20%28single-precision%29))
  (bind _occupyingteam (Variables|Default|GetOccupyingTeam))
  (Networking|SwitchHasAuthority
    (:Authority
      (CallFunction|TickZonesCollisionGameUpdate)
      ;[1 1 1] Update game state so all players can see it
      (bind _assnow_shooter_game_state (Utilities|Casting|CastToSnowShooterGameState (Game|GetGameState)))
      (Utilities|Array|SetArrayElem (Variables|/Script/SnowShooter.SnowShooterGameState|GetFlagOccupiers _assnow_shooter_game_state) (Variables|Default|GetFlagIndex) (Variables|Default|GetOccupyingTeam))
      (Rendering|Material|SetMaterial (Variables|Default|GetCube) 0 (select (== _occupyingteam -1) "/Engine/BasicShapes/BasicShapeMaterial.BasicShapeMaterial" (Utilities|Select :Index _occupyingteam :Option%200 "/Game/SnowShooter/Team1.Team1" :Option%201 "/Game/SnowShooter/Team2.Team2"))))))

(fn ConstructionScript)

(fn TickZonesCollisionGameUpdate
  (for _array_element (Collision|GetOverlappingActors (Variables|Default|GetSphere) "/Script/Engine.Pawn" :!class /Script/Engine.PrimitiveComponent)
    (bind _assnow_shooter_character (Utilities|Casting|CastToSnowShooterCharacter _array_element))
    (if (not (Variables|/Script/SnowShooter.SnowShooterCharacter|GetbIsFrozen _assnow_shooter_character))
      (bind _assnow_shooter_player_state (Utilities|Casting|CastToSnowShooterPlayerState (Variables|/Script/Engine.Pawn|GetPlayerState _assnow_shooter_character)))
      (Math|Integer|IncrementInt (Utilities|Select :Index (Variables|/Script/SnowShooter.SnowShooterPlayerState|GetTeamIndex _assnow_shooter_player_state) :Option%200 (LocalVariables|GetTeam1Count) :Option%201 (LocalVariables|GetTeam2Count)))))
  ;[1 1 1] Capture immediately! TODO: Add timer for other team to take over
  (Math|Integer|CompareInt (LocalVariables|GetTeam1Count) (LocalVariables|GetTeam2Count)
    (:>
      (Variables|Default|SetOccupyingTeam 0))
    (:<
      (Variables|Default|SetOccupyingTeam 1))))